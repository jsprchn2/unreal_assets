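; BP_ObjectSpawner is an actor that spawns one randomly chosen class from its ObjectsToSpawn array at its own location and rotation.
; On BeginPlay it calls AttemptToSpawn, which prints a message if CurrentObject is still valid and otherwise calls SpawnObject.
; SpawnObject picks a random index, spawns at unit scale with adjust-if-possible-but-always-spawn collision handling, and stores the result in CurrentObject.
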(event `self.ReceiveBeginPlay`
  (`self.AttemptToSpawn`))

(fn `AttemptToSpawn`
  (`/Engine/EditorBlueprintResources/StandardMacros.IsValid` (`self.CurrentObject`)
    (:`Is Valid`
      (`KismetSystemLibrary.PrintString` "Object Spawned Already"))
    (:`Is Not Valid`
      (`self.SpawnObject`))))

(fn `SpawnObject`
  (bind _returnvalue (`|SpawnActorFromClass` (`|GetArrayItem` (`self.ObjectsToSpawn`) (`KismetMathLibrary.RandomIntegerInRange` 0 (- (`KismetArrayLibrary.Array_Length` (`self.ObjectsToSpawn`)) 1))) (`KismetMathLibrary.MakeTransform` (`self.K2_GetActorLocation`) (`self.K2_GetActorRotation`)) "AdjustIfPossibleButAlwaysSpawn" "OverrideRootScale" null null))
  (set `self.CurrentObject` _returnvalue))

(fn `UserConstructionScript`)