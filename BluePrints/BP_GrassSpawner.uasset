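; Spawner actor that lays a chain of BP_Grass pieces, starting just below the player pawn when play begins.
; BeginPlay spawns the initial pieces, placing each after the first at the SpawnPoint of the newest one.
; Each piece receives a reference back to the spawner, and SpawnGrassAtSpawnPoint extends the chain from the tracked NewestGrass.
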(event `self.ReceiveBeginPlay`
  (`self.SpawnInitialGrass`))

(fn `SpawnGrass`
  (params (SpawnLocation :type "Vector Structure" :default (0.0 0.0 0.0)))
  (bind _returnvalue (`|SpawnActorFromClass` "/Game/BluePrints/BP_Grass.BP_Grass_C" (`KismetMathLibrary.MakeTransform` SpawnLocation) "Undefined" "OverrideRootScale" null null))
  (bind _output_get (set `self.NewestGrass` _returnvalue))
  (set `/Game/BluePrints/BP_Grass.GrassSpawner` self _output_get))

(fn `SpawnGrassAtSpawnPoint`
  (`self.SpawnGrass` (`SceneComponent.K2_GetComponentLocation` (`/Game/BluePrints/BP_Grass.SpawnPoint` (`self.NewestGrass`)))))

(fn `SpawnInitialGrass`
  (for _ (range 3)
    (`/Engine/EditorBlueprintResources/StandardMacros.IsValid` (`self.NewestGrass`)
      (:`Is Valid`
        (`self.SpawnGrassAtSpawnPoint`))
      (:`Is Not Valid`
        (`self.SpawnGrass` (- (`self.K2_GetActorLocation` (`GameplayStatics.GetPlayerPawn` 0)) (0.0 0.0 120.0)))))))

(fn `UserConstructionScript`)