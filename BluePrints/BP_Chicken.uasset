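; BP_Chicken is a player-controllable chicken pawn with simple hand-rolled movement.
; The moveforward and moveright axes add movement input along actor axes scaled by Speed, and Tick consumes it as a swept, delta-time-scaled local offset.
; The moveforward axis also flips the mesh between two opposite rotations by input sign, with zero taking the negative side, and sets its relative location to the forward vector.
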(event `self.ReceiveTick`
  (params (DeltaSeconds :type "Float (single-precision)"))
  (bind _returnvalue (`self.ConsumeMovementInputVector`))
  (`self.K2_AddActorLocalOffset` (* _returnvalue DeltaSeconds) true))

(event `InputAxis|moveforward`
  (params (AxisValue :type "Float (single-precision)"))
  (bind _returnvalue (`self.GetActorForwardVector`))
  (bind _staticmesh (`self.StaticMesh`))
  (bind _returnvalue_2 (* AxisValue (`self.Speed`)))
  (if (> _returnvalue_2 0.0)
    (`SceneComponent.K2_SetRelativeLocationAndRotation` _staticmesh _returnvalue (struct :`Yaw` 90.0) true false)
    (else
      (`SceneComponent.K2_SetRelativeLocationAndRotation` _staticmesh _returnvalue (struct :`Yaw` 270.0) true false)))
  (`self.AddMovementInput` _returnvalue _returnvalue_2))

(event `InputAxis|moveright`
  (params (AxisValue :type "Float (single-precision)"))
  (`self.AddMovementInput` (`self.GetActorRightVector`) (* AxisValue (`self.Speed`))))

(fn `UserConstructionScript`)