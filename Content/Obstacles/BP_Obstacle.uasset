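; BP_Obstacle is an obstacle actor with a static mesh that removes itself when the player is far away.
; Each tick calls MaybeDespawn, which destroys the actor if player 0's pawn is beyond DespawnDistance.
; The distance check is throttled by DespawnCheckInterval, with the first check delayed by the construction script.
; Any hit on the mesh puts its rigid body to sleep.
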(event `self.ReceiveActorBeginOverlap`
  (params (OtherActor :type "Actor Object Reference")))

(event `self.ReceiveTick`
  (params (DeltaSeconds :type "Float (single-precision)"))
  (`|ExecutionSequence`
    (:`then_0`
      (`self.MaybeDespawn`))))

(event `self.StaticMesh.OnComponentHit`
  (params (HitComponent :type "PrimitiveComponent Object Reference") (OtherActor :type "Actor Object Reference") (OtherComp :type "PrimitiveComponent Object Reference") (NormalImpulse :type "Vector Structure") (Hit :type "HitResult Structure (by ref)"))
  (`PrimitiveComponent.PutRigidBodyToSleep` (`self.StaticMesh`) "None"))

(fn `MaybeDespawn`
  (bind _returnvalue (`KismetSystemLibrary.GetGameTimeInSeconds`))
  (if (> _returnvalue (`self.NextDespawnCheck_Seconds`))
    (set `self.NextDespawnCheck_Seconds` (+ _returnvalue (`self.DespawnCheckInterval`))) ; Only check every so often
    (if (> (`self.GetDistanceTo` (`GameplayStatics.GetPlayerPawn` 0)) (`self.DespawnDistance`))
      (`self.K2_DestroyActor`))))

(fn `UserConstructionScript`
  (set `self.NextDespawnCheck_Seconds` (+ (`KismetSystemLibrary.GetGameTimeInSeconds`) 5.0)))