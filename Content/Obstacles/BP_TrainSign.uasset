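; Railroad crossing sign that warns of nearby trains with flashing lights, a bell and animated arms.
; On Tick it periodically scans all BP_Vehicle actors for trains within separate X and Y distances, using a time-based delay between scans.
; A detected train starts the bell and timed swapping of left/right light meshes; otherwise the light shows green and the bell stops.
; Each state change sets ArmsUp on the arms' animation Blueprint.
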(event `self.ReceiveTick`
  (params (DeltaSeconds :type "Float (single-precision)"))
  (`|ExecutionSequence`
    (:`then_0`
      (`self.ReactToTrains`))
    (:`then_1`
      (`self.FlashingHeartbeat`))))

(fn `AnimationStuffChanged`
  (`|ExecutionSequence`
    (:`then_0`
      (bind _asbp_anim_train_sign (cast `/Game/Obstacles/BP_Anim_TrainSign` (`SkeletalMeshComponent.GetAnimInstance` (`self.Arms`))))
      (set `/Game/Obstacles/BP_Anim_TrainSign.ArmsUp` (not (`self.IsFlashing`)) _asbp_anim_train_sign))))

(fn `FlashingHeartbeat`
  (bind _nextflashtime (`self.NextFlashTime`))
  (bind _crossinglights (`self.CrossingLights`))
  (if (`self.IsFlashing`)
    (if (> (`KismetSystemLibrary.GetGameTimeInSeconds`) _nextflashtime)
      (set `self.NextFlashTime` (+ _nextflashtime (`self.FlashDelay`))) ; Only flash every FlashDelay seconds
      (if (`self.FlashState`)
        (`StaticMeshComponent.SetStaticMesh` _crossinglights "/Game/Assets/Voxel/Terrain/SM_TrainSignFlashLeft.SM_TrainSignFlashLeft")
        (else
          (`StaticMeshComponent.SetStaticMesh` _crossinglights "/Game/Assets/Voxel/Terrain/SM_TrainSignFlashRight.SM_TrainSignFlashRight")))
      (set `self.FlashState` (not (`self.FlashState`))))))

(fn `IsTrainCloseEnough`
  (params (Train :type "/Game/Obstacles/BP_Vehicle Object Reference"))
  (returns (IsCloseEnough :type Boolean))
  (bind (_returnvalue_x _returnvalue_y) (`KismetMathLibrary.BreakVector` (`self.K2_GetActorLocation` Train)))
  (bind (_returnvalue_x_2 _returnvalue_y_2) (`KismetMathLibrary.BreakVector` (`SceneComponent.K2_GetComponentLocation` (`self.DefaultSceneRoot`))))
  (return (and (< (`KismetMathLibrary.Abs` (- _returnvalue_y _returnvalue_y_2)) (`self.ReactionDistanceY`)) (< (`KismetMathLibrary.Abs` (- _returnvalue_x _returnvalue_x_2)) (`self.ReactionDistanceX`)))))

(fn `ReactToTrains`
  (locals (FoundAnything :type Boolean))
  (bind _returnvalue (`KismetSystemLibrary.GetGameTimeInSeconds`))
  (if (< (`self.NextTrainReactionTime`) _returnvalue)
    (set `self.NextTrainReactionTime` (+ _returnvalue (`self.ReactionDelay`))) ; Basically induce a delay between checks
    (`|ExecutionSequence`
      (:`then_0`
        (set `local.FoundAnything` false))
      (:`then_1`
        (bind _outactors (`GameplayStatics.GetAllActorsOfClass` "/Game/Obstacles/BP_Vehicle.BP_Vehicle_C"))
        (for _array_element _outactors
          (if (`/Game/Obstacles/BP_Vehicle.IsTrain` _array_element)
            (bind _iscloseenough (`self.IsTrainCloseEnough` _array_element))
            (if _iscloseenough
              (`|ExecutionSequence`
                (:`then_0`
                  (set `local.FoundAnything` true))
                (:`then_4`
                  (break)))))))
      (:`then_2`
        (if (`local.FoundAnything`)
          (`self.StartFlashing`)
          (else
            (`self.StopFlashing`)))))))

(fn `StartFlashing`
  (if (not (`self.IsFlashing`))
    (set `self.IsFlashing` true)
    (`AudioComponent.Play` (`self.railroad_crossing_bell-Brylon_Terry-1551570865`) 0.0)
    (set `self.NextFlashTime` (`KismetSystemLibrary.GetGameTimeInSeconds`))
    (`self.AnimationStuffChanged`)))

(fn `StopFlashing`
  (`StaticMeshComponent.SetStaticMesh` (`self.CrossingLights`) "/Game/Assets/Voxel/Terrain/SM_TrainSignGreen.SM_TrainSignGreen")
  (set `self.IsFlashing` false)
  (`AudioComponent.Stop` (`self.railroad_crossing_bell-Brylon_Terry-1551570865`))
  (`self.AnimationStuffChanged`))

(fn `UserConstructionScript`)