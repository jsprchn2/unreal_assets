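; BP_Road is a terrain lane actor that spawns moving vehicles and can become a railroad, multilane road or river.
; BeginPlay randomly picks a side, fixing spawn point and travel direction.
; Tick rolls a DeltaSeconds-scaled chance after a minimum delay, spawning BP_Vehicle as a car, train or log.
; Become functions remove the default road and lay mirrored segments; river also retunes spawning, while overlap handling is an empty stub.
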(event `self.ReceiveBeginPlay`
  (`self.Init`))

(event `self.ReceiveActorBeginOverlap`
  (params (OtherActor :type "Actor Object Reference"))
  (`self.HandleOverlap` OtherActor))

(event `self.ReceiveTick`
  (params (DeltaSeconds :type "Float (single-precision)"))
  (`|ExecutionSequence`
    (:`then_0`
      (`self.MaybeSpawnVehicle` DeltaSeconds))))

(fn `BecomeMultilane`
  (if (and (not (`self.IsRailroad`)) true)
    (`|ExecutionSequence`
      (:`then_0`
        (`self.DespawnRoadComponent`))
      (:`then_1`
        (`self.SpawnManyComponentSegments` (`self.Multilane Segments Per Side`) "/Game/Assets/Voxel/Terrain/SM_Road_With_Lanes.SM_Road_With_Lanes" (`self.Multilane Segment Spacing`) (`self.Multilane Segment Scale`) (struct :`Yaw` 90.0))))))

(fn `BecomeRailroad`
  (`|ExecutionSequence`
    (:`then_0`
      (`self.DespawnRoadComponent`))
    (:`then_1`
      (set `self.IsRailroad` true))
    (:`then_2`
      (`self.SpawnManyComponentSegments` (`self.TrackSegmentsPerSide`) "/Game/Assets/Voxel/Terrain/SM_TrainTrack.SM_TrainTrack" (`self.TrackSegmentsSpacing`) (`self.TrainTrackScale`) (struct :`Yaw` 90.0) (0.0 0.0 -4.0)))
    (:`then_3`
      (`self.SpawnManyActorSegments` (`self.TrainTrackSignSegmentsPerSide`) (`self.TrainTrackSignSegmentSpacing`) (1.0 1.0 1.0) (struct :`Yaw` 90.0) (`self.TrainTrackSignSegmentTransform`) "/Game/Obstacles/BP_TrainSign.BP_TrainSign_C"))))

(fn `BecomeRiver`
  (`|ExecutionSequence`
    (:`then_0`
      (`self.DespawnRoadComponent`))
    (:`then_1`
      (set `self.IsRiver` true)
      (set `self.Spawn Vehicle Chance` (`self.RiverSpawnLogChance`)))
    (:`then_2`
      ;[1 1 1] Spawn water components, wewt
      (`self.SpawnManyActorSegments` (`self.RiverSegmentsPerSide`) (`self.RiverSegmentsSpacing`) (`self.RiverSegmentScale`) (struct) (0.0 0.0 3.0) "/Game/Terrain/BP_RiverSegment.BP_RiverSegment_C"))
    (:`then_3`
      (set `self.SpawnDelay_Seconds` (`self.DefaultRiverSpawnDelay_Seconds`)))))

(fn `CheckAnyTrainsCloseToSign`)

(fn `CheckSpawnDelay`
  (returns (CanSpawn :type Boolean))
  (return (> (`KismetSystemLibrary.GetGameTimeInSeconds`) (`self.NextSpawn_MinimumGameTime`))))

(fn `DespawnRoadComponent`
  (bind _road (`self.Road`))
  (if (`KismetSystemLibrary.IsValid` _road)
    (`ActorComponent.K2_DestroyComponent` _road)))

(fn `HandleOverlap`
  (params (OtherActor :type "Actor Object Reference")))

(fn `Init`
  (`|ExecutionSequence`
    (:`then_0`
      (`self.InitRandomSpawnPoint`))))

(fn `InitRandomSpawnPoint`
  (if (`KismetMathLibrary.RandomBool`)
    (set `self.ActiveSpawnPoint` (`SceneComponent.K2_GetComponentLocation` (`self.SpawnPoint_Left`)))
    (set `self.SpawnVehicleDirectionY` 1.0)
    (set `self.SpawnVehicleRotation` (struct :`Yaw` 180.0))
    (else
      (set `self.ActiveSpawnPoint` (`SceneComponent.K2_GetComponentLocation` (`self.SpawnPoint_Right`)))
      (set `self.SpawnVehicleDirectionY` -1.0)
      (set `self.SpawnVehicleRotation` (struct)))))

(fn `IsRoad`
  (returns (IsRoad :type Boolean))
  (return (and (not (`self.IsRailroad`)) true)))

(fn `MaybeSpawnVehicle`
  (params (DeltaSeconds :type "Float (double-precision)"))
  (bind _canspawn (`self.CheckSpawnDelay`))
  (if _canspawn
    (if (> (* DeltaSeconds (`self.Spawn Vehicle Chance`)) (`KismetMathLibrary.RandomFloat`))
      (`self.SpawnVehicle`))))

(fn `ResetSpawnDelay`
  (set `self.NextSpawn_MinimumGameTime` (+ (`KismetSystemLibrary.GetGameTimeInSeconds`) (`self.SpawnDelay_Seconds`))))

(fn `SpawnManyActorSegments`
  (params (CountPerSide :type Integer) (Spacing :type "Float (double-precision)") (Scale :type "Vector Structure") (Rotation :type "Rotator Structure") (AddLocationTransform :type "Vector Structure") (ActorClass :type "Actor Class Reference"))
  (locals (SpawnedComponents :type "/DatasmithContent/Blueprints/FBXImporter/ArrayOfActor Structure"))
  (bind (_returnvalue_x _returnvalue_y _returnvalue_z) (`KismetMathLibrary.BreakVector` (+ AddLocationTransform (`SceneComponent.K2_GetComponentLocation` (`self.DefaultSceneRoot`)))))
  (`|ExecutionSequence`
    (:`then_0`
      (for _index (range (* CountPerSide -1) (+ CountPerSide 1))
        (bind _returnvalue (`|SpawnActorFromClass` ActorClass (`KismetMathLibrary.MakeTransform` (`KismetMathLibrary.MakeVector` (+ 0.0 _returnvalue_x) (+ (* _index Spacing) _returnvalue_y) (+ 0.0 _returnvalue_z)) Rotation Scale) "Undefined" "OverrideRootScale" null null))))))

(fn `SpawnManyComponentSegments`
  (params (CountPerSide :type Integer) (StaticMesh :type "StaticMesh Object Reference") (Spacing :type "Float (double-precision)") (Scale :type "Vector Structure") (Rotation :type "Rotator Structure") (AddLocationTransform :type "Vector Structure") (GenerateOverlap :type Boolean))
  (locals (SpawnedComponents :type "/DatasmithContent/Blueprints/FBXImporter/ArrayOfActor Structure"))
  (`|ExecutionSequence`
    (:`then_0`
      (for _index (range (* CountPerSide -1) (+ CountPerSide 1))
        (bind _returnvalue (`AddComponent|NODE_AddStaticMeshComponent-2` :`RelativeTransform` (`KismetMathLibrary.MakeTransform` (`KismetMathLibrary.MakeVector` 0.0 (* _index Spacing) 5.0) Rotation Scale)))
        (`|ExecutionSequence`
          (:`then_0`
            (`StaticMeshComponent.SetStaticMesh` _returnvalue StaticMesh)
            (`SceneComponent.K2_AddRelativeLocation` _returnvalue AddLocationTransform false false))
          (:`then_1`
            (if true
              (set `PrimitiveComponent.bGenerateOverlapEvents` true _returnvalue))))))))

(fn `SpawnVehicle`
  (`|ExecutionSequence`
    (:`then_0`
      (bind _returnvalue (`|SpawnActorFromClass` "/Game/Obstacles/BP_Vehicle.BP_Vehicle_C" (`KismetMathLibrary.MakeTransform` (`self.ActiveSpawnPoint`)) "Undefined" "OverrideRootScale" null null))
      (set `/Game/Obstacles/BP_Vehicle.VelocityDirection` (`KismetMathLibrary.MakeVector` 0.0 (`self.SpawnVehicleDirectionY`)) _returnvalue) ; Set the Vehicle's Initial Velocity
      (`/Game/Obstacles/BP_Vehicle.SetRotation` _returnvalue (`self.SpawnVehicleRotation`)) ; Make sure the vehicle is facing the right direction,\nper what InitRandomSpawnPoint decided
      (if (`self.IsRailroad`)
        (`/Game/Obstacles/BP_Vehicle.BecomeTrain` _returnvalue)
        (elif (`self.IsRiver`)
          (`/Game/Obstacles/BP_Vehicle.BecomeLog` _returnvalue))))
    (:`then_1`
      (`self.ResetSpawnDelay`))))

(fn `UserConstructionScript`
  (`|ExecutionSequence`
    (:`then_0`
      (set `self.SpawnDelay_Seconds` (`self.DefaultMinimumSpawnDelay_Seconds`)))
    (:`then_1`
      (set `self.Spawn Vehicle Chance` (`self.DefaultSpawnVehicleChance`)))))