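; BP_StartScreen is a start screen actor whose Main component slides in toward its relative origin.
; The construction script sets SlidingIn, and Tick then eases Main toward zero by a distance-proportional step scaled by SlideFactor and delta time.
; MaybeDoneSlidingIn would clear the flag below a threshold but is not called here.
; IsDoneSlidingIn returns SlidingIn directly, so true means still sliding, contrary to its name.
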(event `self.ReceiveTick`
  (params (DeltaSeconds :type "Float (single-precision)"))
  (`self.SlideIn_Heartbeat` DeltaSeconds))

(fn `IsDoneSlidingIn`
  (returns (IsDone :type Boolean))
  (return (`self.SlidingIn`)))

(fn `MaybeDoneSlidingIn`
  (bind (_relativelocation_x _relativelocation_y _relativelocation_z) (`KismetMathLibrary.BreakVector` (`SceneComponent.RelativeLocation` (`self.Main`))))
  (if (and (< _relativelocation_x 1.0) (< _relativelocation_y 1.0) (< _relativelocation_z 1.0))
    (`|ExecutionSequence`
      (:`then_0`
        (set `self.SlidingIn` false)))))

(fn `SlideIn_Heartbeat`
  (params (DeltaSeconds :type "Float (double-precision)"))
  (bind _main (`self.Main`))
  (bind _slidefactor (`self.SlideFactor`))
  (bind (_relativelocation_x _relativelocation_y _relativelocation_z) (`KismetMathLibrary.BreakVector` (`SceneComponent.RelativeLocation` _main)))
  (if (`self.SlidingIn`)
    (`SceneComponent.K2_SetRelativeLocation` _main (`KismetMathLibrary.MakeVector` (- _relativelocation_x (* (/ _relativelocation_x _slidefactor) DeltaSeconds)) (- _relativelocation_y (* (/ _relativelocation_y _slidefactor) DeltaSeconds)) (- _relativelocation_z (* (/ _relativelocation_z _slidefactor) DeltaSeconds))) false false)))

(fn `StartSlidingIn`
  (`|ExecutionSequence`
    (:`then_0`
      (set `self.SlidingIn` true))))

(fn `UserConstructionScript`
  (`|ExecutionSequence`
    (:`then_0`
      (`self.StartSlidingIn`))))