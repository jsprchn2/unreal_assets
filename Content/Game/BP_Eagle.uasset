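; Eagle hazard that hunts the player, carries them off screen and marks them dead.
; BeginChasingPlayer places it at an offset from the player; Tick then homes in, with constant X speed and distance-scaled Y/Z movement.
; Overlapping BP_Player snaps the pawn beneath it and lifts both with growing upward velocity.
; Death triggers once the eagle has not been rendered recently, while its screech audio is kept playing throughout.
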(event `self.ReceiveTick`
  (params (DeltaSeconds :type "Float (single-precision)"))
  (`|ExecutionSequence`
    (:`then_0`
      (`self.ChasePlayer` DeltaSeconds))
    (:`then_1`
      (`self.LiftPlayer` DeltaSeconds))
    (:`then_2`
      (`self.CheckDoneLiftingPlayer`))
    (:`then_3`
      (`self.EnsureAudioPlaying`))))

(event `self.ReceiveActorBeginOverlap`
  (params (OtherActor :type "Actor Object Reference"))
  (cast `/Game/Player/BP_Player` OtherActor)
  (`self.Begin Lifting Player`))

(fn `Begin Lifting Player`
  (`|ExecutionSequence`
    (:`then_0`
      (set `self.IsChasingPlayer` false)
      (set `self.IsLiftingPlayer` true))
    (:`then_1`
      (`SceneComponent.K2_SetWorldLocation` (`Actor.RootComponent` (`GameplayStatics.GetPlayerPawn` 0)) (+ (`self.K2_GetActorLocation`) (-10.0 0.0 -15.0)) false false))))

(fn `BeginChasingPlayer`
  (params (Player :type "/Game/Player/BP_Player Object Reference"))
  (`|ExecutionSequence`
    (:`then_0`
      (set `self.IsChasingPlayer` true)
      (set `self.IsLiftingPlayer` false))
    (:`then_1`
      (`SceneComponent.K2_SetWorldLocation` (`self.DefaultSceneRoot`) (+ (`self.K2_GetActorLocation` Player) (`self.InitialOffsetToPlayer`)) false false))))

(fn `ChasePlayer`
  (params (DeltaTime :type "Float (double-precision)"))
  (locals (YAmount :type "Float (double-precision)"))
  (bind _speed (`self.Speed`))
  (bind _chaseplayersmoothingfactor (`self.ChasePlayerSmoothingFactor`))
  (bind (_returnvalue_x _returnvalue_y _returnvalue_z) (`KismetMathLibrary.BreakVector` (`self.K2_GetActorLocation` (`GameplayStatics.GetPlayerPawn` 0))))
  (bind (_returnvalue_x_2 _returnvalue_y_2 _returnvalue_z_2) (`KismetMathLibrary.BreakVector` (`SceneComponent.K2_GetComponentLocation` (`self.DefaultSceneRoot`))))
  (if (`self.IsChasingPlayer`)
    (`|ExecutionSequence`
      (:`then_0`
        (if (> _returnvalue_x _returnvalue_x_2)
          (set `self.XDirection` 1.0)
          (else
            (set `self.XDirection` -1.0))))
      (:`then_1`
        (`SceneComponent.K2_AddWorldOffset` (`self.DefaultSceneRoot`) (`KismetMathLibrary.MakeVector` (* DeltaTime _speed (`self.XDirection`)) (* _speed DeltaTime (/ (- _returnvalue_y _returnvalue_y_2) _chaseplayersmoothingfactor)) (* _speed DeltaTime (/ (- _returnvalue_z _returnvalue_z_2) _chaseplayersmoothingfactor))) false false)))))

(fn `CheckDoneLiftingPlayer`
  (if (and (`self.IsLiftingPlayer`) (not (`self.WasRecentlyRendered` 0.2)))
    (`self.HandleDoneLiftingPlayer`)))

(fn `EnsureAudioPlaying`
  (bind _hawk_screeching_mike_koenig_1626170357 (`self.Hawk_Screeching-Mike_Koenig-1626170357`))
  (if (not (`AudioComponent.IsPlaying` _hawk_screeching_mike_koenig_1626170357))
    (`AudioComponent.Play` _hawk_screeching_mike_koenig_1626170357 0.0)))

(fn `HandleDoneLiftingPlayer`
  (bind _asbp_player (cast `/Game/Player/BP_Player` (`GameplayStatics.GetPlayerPawn` 0)))
  (set `/Game/Player/BP_Player.IsDead` true _asbp_player))

(fn `LiftPlayer`
  (params (DeltaSeconds :type "Float (double-precision)"))
  (bind _speed (`self.Speed`))
  (bind _liftvelocity (`self.LiftVelocity`))
  (bind _returnvalue (* DeltaSeconds _liftvelocity _speed))
  (bind _returnvalue_2 (* DeltaSeconds (`self.XDirection`) _speed))
  (if (`self.IsLiftingPlayer`)
    (`|ExecutionSequence`
      (:`then_0`
        (`SceneComponent.K2_AddWorldOffset` (`self.DefaultSceneRoot`) (`KismetMathLibrary.MakeVector` _returnvalue_2 0.0 _returnvalue) false false)
        (`SceneComponent.K2_AddWorldOffset` (`Actor.RootComponent` (`GameplayStatics.GetPlayerPawn` 0)) (`KismetMathLibrary.MakeVector` _returnvalue_2 0.0 _returnvalue) false false))
      (:`then_1`
        (set `self.LiftVelocity` (+ _liftvelocity DeltaSeconds))))))

(fn `UserConstructionScript`
  (`|ExecutionSequence`
    (:`then_0`
      (`self.EnsureAudioPlaying`))))