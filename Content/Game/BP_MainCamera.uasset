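; BP_MainCamera is the game's main camera, which scrolls automatically, stays up with the player and can frame a start screen.
; Each tick it snaps forward on X if it falls below a minimum offset from the player, then moves by ScrollSpeed while scrolling is enabled.
; It aims at the player on BeginPlay.
; Other functions toggle scrolling, take the view target, realign to the player, or position and aim it at the start screen.
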(event `self.ReceiveBeginPlay`
  (`self.FaceThePlayer`))

(event `self.ReceiveTick`
  (params (DeltaSeconds :type "Float (single-precision)"))
  (`|ExecutionSequence`
    (:`then_0`
      (`self.CatchUpWithPlayer`))
    (:`then_1`
      (`self.MaybeDoScroll` DeltaSeconds))))

(fn `AlignToPlayer`
  (`SceneComponent.K2_SetWorldLocation` (`self.DefaultSceneRoot`) (+ (`self.K2_GetActorLocation` (`GameplayStatics.GetPlayerPawn` 0)) (`self.DefaultOffsetToPlayer`)) false false))

(fn `CatchUpWithPlayer`
  (bind _returnvalue (`GameplayStatics.GetPlayerPawn` 0))
  (bind (_returnvalue_x _returnvalue_y _returnvalue_z) (`KismetMathLibrary.BreakVector` (`SceneComponent.K2_GetComponentLocation` (`self.DefaultSceneRoot`))))
  (bind _returnvalue_x_2 (`KismetMathLibrary.BreakVector` (`SceneComponent.K2_GetComponentLocation` (`Actor.RootComponent` _returnvalue))))
  (bind _returnvalue_2 (+ (`self.MinimumOffsetToPlayer`) _returnvalue_x_2))
  (if (`KismetSystemLibrary.IsValid` _returnvalue)
    (if (< _returnvalue_x _returnvalue_2)
      (`SceneComponent.K2_SetWorldLocation` (`self.DefaultSceneRoot`) (`KismetMathLibrary.MakeVector` _returnvalue_2 _returnvalue_y _returnvalue_z) false true))))

(fn `DoScroll`
  (params (DeltaSeconds :type "Float (double-precision)"))
  (bind _defaultsceneroot (`self.DefaultSceneRoot`))
  (`SceneComponent.K2_SetWorldLocation` _defaultsceneroot (+ (`SceneComponent.K2_GetComponentLocation` _defaultsceneroot) (* (`self.ScrollSpeed`) DeltaSeconds)) false false))

(fn `DoStartScreen`
  (params (StartScreen :type "/Game/Game/BP_StartScreen Object Reference"))
  (`|ExecutionSequence`
    (:`then_0`
      (`self.StopScrolling`))
    (:`then_1`
      (`self.PositionForStartScreen` StartScreen))
    (:`then_2`
      (`self.FaceStartScreen` StartScreen))))

(fn `FaceActor`
  (params (Actor :type "Actor Object Reference"))
  (bind _camera (`self.Camera`))
  (if (`KismetSystemLibrary.IsValid` Actor)
    (`|ExecutionSequence`
      (:`then_0`
        (`SceneComponent.K2_SetWorldRotation` _camera (`KismetMathLibrary.Conv_VectorToRotator` (`KismetMathLibrary.GetDirectionUnitVector` (`SceneComponent.K2_GetComponentLocation` _camera) (`self.K2_GetActorLocation` Actor))) false false)))))

(fn `FaceStartScreen`
  (params (StartScreen :type "/Game/Game/BP_StartScreen Object Reference"))
  (`self.FaceActor` StartScreen))

(fn `FaceThePlayer`
  (bind _camera (`self.Camera`))
  (if (`KismetSystemLibrary.IsValid` (`GameplayStatics.GetPlayerPawn` 0))
    (`|ExecutionSequence`
      (:`then_0`
        (`self.CatchUpWithPlayer`))
      (:`then_1`
        (`SceneComponent.K2_SetWorldRotation` _camera (`KismetMathLibrary.Conv_VectorToRotator` (`KismetMathLibrary.GetDirectionUnitVector` (`SceneComponent.K2_GetComponentLocation` _camera) (`SceneComponent.K2_GetComponentLocation` (`Actor.RootComponent` (`GameplayStatics.GetPlayerPawn` 0))))) false false) ; Rotate camera to face the player
      ))))

(fn `MaybeDoScroll`
  (params (DeltaSeconds :type "Float (double-precision)"))
  (if (`self.CanDoScroll`)
    (`self.DoScroll` DeltaSeconds)))

(fn `PositionForStartScreen`
  (params (StartScreen :type "/Game/Game/BP_StartScreen Object Reference"))
  (`self.K2_SetActorLocation` (+ (`self.K2_GetActorLocation` StartScreen) (`self.OffsetToStartScreen`))))

(fn `StartScrolling`
  (set `self.CanDoScroll` true))

(fn `StopScrolling`
  (set `self.CanDoScroll` false))

(fn `TakeView`
  (returns (Done :type Boolean))
  (`PlayerController.SetViewTargetWithBlend` (`GameplayStatics.GetPlayerController` 0) self 0.0 "VTBlend_Linear" 0.0 false)
  (return false))

(fn `UserConstructionScript`
  (`|ExecutionSequence`
    (:`then_0`
      (`self.StopScrolling`))
    (:`then_1`
      (`SceneComponent.K2_SetWorldLocation` (`self.DefaultSceneRoot`) (`self.DefaultOffsetToPlayer`) false false))))