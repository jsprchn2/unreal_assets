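; BP_SideCamera is a camera actor that follows the player pawn from a fixed offset, mostly along the Y axis, for a side-on view.
; Every Tick it moves its Camera component to the pawn's location plus that offset, if a pawn exists, then rotates it to face the pawn.
; A separate TakeView function sets this actor as player 0's view target, but nothing in this Blueprint calls it.
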(event `self.ReceiveTick`
  (params (DeltaSeconds :type "Float (single-precision)"))
  (`self.FollowThePlayer`))

(fn `FaceThePlayer`
  (bind _camera (`self.Camera`))
  (`SceneComponent.K2_SetWorldRotation` _camera (`KismetMathLibrary.Conv_VectorToRotator` (`KismetMathLibrary.GetDirectionUnitVector` (`SceneComponent.K2_GetComponentLocation` _camera) (`SceneComponent.K2_GetComponentLocation` (`Actor.RootComponent` (`GameplayStatics.GetPlayerPawn` 0))))) false false))

(fn `FollowThePlayer`
  (bind _returnvalue (`GameplayStatics.GetPlayerPawn` 0))
  (bind (_returnvalue_x _returnvalue_y _returnvalue_z) (`KismetMathLibrary.BreakVector` (`self.K2_GetActorLocation` _returnvalue)))
  (if (`KismetSystemLibrary.IsValid` _returnvalue)
    (`SceneComponent.K2_SetWorldLocation` (`self.Camera`) (`KismetMathLibrary.MakeVector` (+ _returnvalue_x 0.0) (+ _returnvalue_y 50.0) (+ _returnvalue_z 1.0)) false false)
    (`self.FaceThePlayer`)))

(fn `TakeView`
  (returns (Done :type Boolean))
  (`PlayerController.SetViewTargetWithBlend` (`GameplayStatics.GetPlayerController` 0) self 0.0 "VTBlend_Linear" 0.0 false)
  (return false))

(fn `UserConstructionScript`)